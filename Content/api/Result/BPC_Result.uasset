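; Actor component or Blueprint that holds a result widget and pops it up on an emergency signal.
; On BeginPlay it registers itself as the target (타깃) variable on the player's BP_FirstPersonCharacter.
; Its PopUpEmergency event unhides the ResultWidget component when that widget is not already visible.
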(event Custom|PopUpEmergency
  (if (not (Class|WidgetComponent|IsWidgetVisible (Variables|Default|GetResultWidget)))
    (Development|SetHiddeninGame (Variables|Default|GetResultWidget) false false)))

(event EventBeginPlay
  (Variables|/Game/FirstPerson/Blueprints/BP_FirstPersonCharacter.BP_FirstPersonCharacter_C|Set타깃 (.AsBP%20First%20Person%20Character (Utilities|Casting|CastToBP_FirstPersonCharacter (Game|GetPlayerCharacter 0))) self))

(fn ConstructionScript)